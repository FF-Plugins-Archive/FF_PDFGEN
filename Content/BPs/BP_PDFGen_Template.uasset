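; Test Blueprint for the PDFGen plugin that builds and saves a sample PDF on BeginPlay.
; It creates a document with metadata, adds colored text and an image, then saves to a hard-coded, platform-specific path on Windows or Android and closes it.
; Failed steps print the stage name, and a successful save prints the close result.
; A separate PDFGen_Nodes graph holds unconnected example nodes.
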(event `self.ReceiveBeginPlay`
  (bind _out_pdf (`FF_PDFGENBPLibrary.PDFGen_Doc_Create` "Eray" "UE5 Creator" (`KismetMathLibrary.Now`) "UE5 Producer" "PDFGen Test" "PDFGen Test Title" (1920.0 1080.0)))
  (bind _output_get (set `self.REF_Doc_PDFGen` _out_pdf))
  (bind _returnvalue (`FF_PDFGENBPLibrary.PDFGen_Add_Text` _output_get 0 "Eray" (50.0 20.0) (0.0 0.0) 16.0 (make `Color` 255)))
  (if _returnvalue
    (bind _returnvalue_2 (`FF_PDFGENBPLibrary.PDFGen_Add_Image` (`self.REF_Doc_PDFGen`) 0 "/Engine/Tutorial/Mobile/TutorialAssets/android_Icon.android_Icon" (200.0 200.0)))
    (if _returnvalue_2
      (switch `string` (`GameplayStatics.GetPlatformName`)
        (:`Windows`
          (bind _returnvalue_3 (`FF_PDFGENBPLibrary.PDFGen_Doc_Save` (`self.REF_Doc_PDFGen`) (`KismetSystemLibrary.NormalizeFilename` "C:\\Users\\erayo\\Downloads\\sample_pdfgen.pdf")))
          (if _returnvalue_3
            (bind _returnvalue_4 (`FF_PDFGENBPLibrary.PDFGen_Doc_Close` (`self.REF_Doc_PDFGen`) :!label _label))
            (`KismetSystemLibrary.PrintString` (`KismetStringLibrary.Conv_BoolToString` _returnvalue_4))
            (else
              (`KismetSystemLibrary.PrintString` "Save" :!label _label_2))))
        (:`Android`
          (bind _returnvalue_5 (`FF_PDFGENBPLibrary.PDFGen_Doc_Save` (`self.REF_Doc_PDFGen`) (`ExtendedVarsBPLibrary.Android_Path_Helper` "Download/sample_pdfgen.pdf")))
          (if _returnvalue_5
            (goto _label)
            (else
              (goto _label_2)))))
      (else
        (`KismetSystemLibrary.PrintString` "Add Image")))
    (else
      (`KismetSystemLibrary.PrintString` "Add Text"))))

(fn `UserConstructionScript`)